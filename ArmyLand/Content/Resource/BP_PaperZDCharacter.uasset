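; Player-controlled PaperZD 2D character with left/right movement, jumping and a simple lives count.
; BeginPlay adds the Enhanced Input mapping, caches the Player_AnimBP instance and adds the WB_PaperHUD widget to the viewport.
; Movement follows the control rotation's forward vector and flips the sprite by rotation, while jump input also sets the animation's IsJumpig flag.
; TakeDamage subtracts from Lives and only prints the remaining count, or "Dead" at exactly zero.
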(event `self.ReceiveBeginPlay`
  (bind _asplayer_controller (cast `PlayerController` (`self.GetController`)))
  (bind _returnvalue (pcsubsystem `EnhancedInputLocalPlayerSubsystem` _asplayer_controller))
  (`/Engine/EditorBlueprintResources/StandardMacros.IsValid` _returnvalue
    (:`Is Valid`
      (`EnhancedInputSubsystemInterface.AddMappingContext` _returnvalue "/Game/Resource/Inputs/MC_Map.MC_Map" 0 (struct))
      (bind _asplayer_anim_bp (cast `/Game/Resource/Player_AnimBP` (`PaperZDAnimationComponent.AnimInstance` (`self.AnimationComponent`))))
      (set `self.As Player Anim BP` _asplayer_anim_bp)
      (bind _returnvalue_2 (`|CreateWidget` "/Game/Resource/HUD/WB_PaperHUD.WB_PaperHUD_C"))
      (bind _output_get (set `self.HUD` _returnvalue_2))
      (`UserWidget.AddToViewport` _output_get 0))))

(event `EnhancedInput|/Game/Resource/Inputs/IA_Movement`
  (params (ActionValue :type "Float (double-precision)") (ElapsedSeconds :type "Float (double-precision)") (TriggeredSeconds :type "Float (double-precision)") (InputAction :type "InputAction Object Reference" :default "/Game/Resource/Inputs/IA_Movement.IA_Movement"))
  (bind (_returnvalue_roll _returnvalue_pitch _returnvalue_yaw) (`KismetMathLibrary.BreakRotator` (`self.GetControlRotation` (`GameplayStatics.GetPlayerPawn` 0))))
  ; Move left/right
  (:`Triggered`
    (`self.AddMovementInput` (`KismetMathLibrary.GetForwardVector` (`KismetMathLibrary.MakeRotator` _returnvalue_roll 0.0 _returnvalue_yaw)) ActionValue)
    ; Flips Sprite
    (if (> ActionValue 0.0)
      (`SceneComponent.K2_SetRelativeRotation` :`self` (`self.Sprite`))
      (elif (< ActionValue 0.0)
        (`SceneComponent.K2_SetRelativeRotation` (`self.Sprite`) (struct :`Yaw` -180.0) false false)))))

(event `EnhancedInput|/Game/Resource/Inputs/IA_Jump`
  (params (ActionValue :type "Float (double-precision)") (ElapsedSeconds :type "Float (double-precision)") (TriggeredSeconds :type "Float (double-precision)") (InputAction :type "InputAction Object Reference" :default "/Game/Resource/Inputs/IA_Jump.IA_Jump"))
  ; Allows Player to jump
  (:`Triggered`
    (`self.Jump`)
    (set `/Game/Resource/Player_AnimBP.IsJumpig ` true (`self.As Player Anim BP`)))
  (:`Completed`
    (`self.StopJumping`)
    (set `/Game/Resource/Player_AnimBP.IsJumpig ` false (`self.As Player Anim BP`))))

(fn `TakeDamage`
  (params (Damage :type Integer))
  (bind _output_get (set `self.Lives` (- (`self.Lives`) Damage)))
  (if (== _output_get 0)
    (`KismetSystemLibrary.PrintString` "Dead")
    (else
      (`KismetSystemLibrary.PrintString` (`KismetStringLibrary.Conv_IntToString` _output_get)))))

(fn `UserConstructionScript`)
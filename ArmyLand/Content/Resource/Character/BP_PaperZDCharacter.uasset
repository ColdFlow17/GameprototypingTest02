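; Player PaperZD character for a 2D game, handling movement, jumping, shooting, reloading and lives.
; BeginPlay adds the Enhanced Input mapping, caches the anim Blueprint for the jump flag and creates the HUD; movement flips the sprite.
; Firing decrements ammo twice, runs an unused line trace and spawns BP_Bullet; reload decrements Reloads without refilling ammo.
; Ammo changes notify through CallEUpdateAmmo; TakeDamage updates HUD lives, pausing on game over at zero.
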(event `self.ReceiveBeginPlay`
  (bind _asplayer_controller (cast `PlayerController` (`self.GetController`)))
  (bind _returnvalue (pcsubsystem `EnhancedInputLocalPlayerSubsystem` _asplayer_controller))
  (`/Engine/EditorBlueprintResources/StandardMacros.IsValid` _returnvalue
    (:`Is Valid`
      (`EnhancedInputSubsystemInterface.AddMappingContext` _returnvalue "/Game/Resource/Inputs/MC_Map.MC_Map" 0 (struct))
      (bind _asplayer_anim_bp (cast `/Game/Resource/Player_AnimBP` (`PaperZDAnimationComponent.AnimInstance` (`self.AnimationComponent`))))
      (set `self.As Player Anim BP` _asplayer_anim_bp)
      (bind _returnvalue_2 (`|CreateWidget` "/Game/Resource/HUD/WB_PaperHUD.WB_PaperHUD_C"))
      (bind _output_get (set `self.HUD` _returnvalue_2))
      (`UserWidget.AddToViewport` _output_get 0)
      (`/Game/Resource/HUD/WB_PaperHUD.InitializeHUD` _output_get self))))

(event `EnhancedInput|/Game/Resource/Inputs/IA_Movement`
  (params (ActionValue :type "Float (double-precision)") (ElapsedSeconds :type "Float (double-precision)") (TriggeredSeconds :type "Float (double-precision)") (InputAction :type "InputAction Object Reference" :default "/Game/Resource/Inputs/IA_Movement.IA_Movement"))
  (bind (_returnvalue_roll _returnvalue_pitch _returnvalue_yaw) (`KismetMathLibrary.BreakRotator` (`self.GetControlRotation` (`GameplayStatics.GetPlayerPawn` 0))))
  ; Move left/right
  (:`Triggered`
    (`self.AddMovementInput` (`KismetMathLibrary.GetForwardVector` (`KismetMathLibrary.MakeRotator` _returnvalue_roll 0.0 _returnvalue_yaw)) ActionValue)
    ; Flips Sprite
    (if (> ActionValue 0.0)
      (`SceneComponent.K2_SetRelativeRotation` :`self` (`self.Sprite`))
      (elif (< ActionValue 0.0)
        (`SceneComponent.K2_SetRelativeRotation` (`self.Sprite`) (struct :`Yaw` -180.0) false false)))))

(event `self.OnLanded`
  (params (Hit :type "HitResult Structure (by ref)"))
  (`self.StopJumping`)
  (set `/Game/Resource/Player_AnimBP.IsJumpig ` false (`self.As Player Anim BP`))
  (goto _label :!via `Reset`))

(event `EnhancedInput|/Game/Resource/Inputs/IA_Jump`
  (params (ActionValue :type "Float (double-precision)") (ElapsedSeconds :type "Float (double-precision)") (TriggeredSeconds :type "Float (double-precision)") (InputAction :type "InputAction Object Reference" :default "/Game/Resource/Inputs/IA_Jump.IA_Jump"))
  ; Allows Player to jump
  (:`Started`
    (`self.Jump`)
    (set `/Game/Resource/Player_AnimBP.IsJumpig ` true (`self.As Player Anim BP`))
    (`/Engine/EditorBlueprintResources/StandardMacros.DoOnce` (stale _output_get) :!label _label
      (:`Completed`
        (`TypedElementListLibrary.Reset` (struct)))))
  (:`Completed`
    (`self.StopJumping`)
    (bind _output_get (set `/Game/Resource/Player_AnimBP.IsJumpig ` false (`self.As Player Anim BP`)))))

(event `EnhancedInput|/Game/Resource/Inputs/IA_Attack`
  (params (ActionValue :type Boolean) (ElapsedSeconds :type "Float (double-precision)") (TriggeredSeconds :type "Float (double-precision)") (InputAction :type "InputAction Object Reference" :default "/Game/Resource/Inputs/IA_Attack.IA_Attack"))
  (bind _bulle_spawn (`self.bulle spawn`))
  (:`Started`
    (if (>= (`self.Ammo`) 1)
      (bind _result (`/Engine/EditorBlueprintResources/StandardMacros.DecrementInt` (`self.Ammo`))
        (:`  `
          (set `self.CurrentMagAmmo` _result)
          (`self.LineTraceForShooting`)
          (`KismetSystemLibrary.PrintText` "shoot")
          (`|SpawnActorFromClass` "/Game/Resource/BP_Bullet.BP_Bullet_C" (`KismetMathLibrary.MakeTransform` (`SceneComponent.K2_GetComponentLocation` _bulle_spawn) (`SceneComponent.K2_GetComponentRotation` _bulle_spawn)) "Undefined" "MultiplyWithRoot" null null)
          (`self.E_UpdateAmmo` (`self.CurrentMagAmmo`) (`self.CurrentReserveAmmo`))))
      (else
        (`KismetSystemLibrary.PrintString` "No Ammo")))))

(event `EnhancedInput|/Game/Resource/Inputs/IA_Reload`
  (params (ActionValue :type Boolean) (ElapsedSeconds :type "Float (double-precision)") (TriggeredSeconds :type "Float (double-precision)") (InputAction :type "InputAction Object Reference" :default "/Game/Resource/Inputs/IA_Reload.IA_Reload"))
  (:`Triggered`
    (set `self.set relaod` true)
    (if (<= 0 (`self.Ammo`))
      (bind _output_get (set `self.reloads` (- (`self.reloads`) 1)))
      (set `self.reloads` _output_get)
      (bind _output_get_2 (set `self.Ammo` (`self.Ammo`)))
      (bind _output_get_3 (set `self.CurrentMagAmmo` _output_get_2))
      (bind _output_get_4 (set `self.CurrentReserveAmmo` _output_get_2))
      (`self.E_UpdateAmmo` _output_get_3 _output_get_4)
      (set `self.set relaod` true)
      (if (<= (`self.reloads`) 0)
        (set `self.set relaod` false)
        (set `self.reloads` 0)
        (`KismetSystemLibrary.PrintString` "no relaod ")))))

(event `UpdateAmmo`
  (params (CurrentMagAmmo :type Integer) (CurrenrReserveAmmo :type Integer))
  (`self.E_UpdateAmmo` CurrentMagAmmo CurrenrReserveAmmo))

(fn `DeathOperation`
  (bind _returnvalue (`GameplayStatics.GetPlayerController` 0))
  (`GameplayStatics.SetGamePaused` true)
  (set `PlayerController.bShowMouseCursor` true _returnvalue)
  (`WidgetBlueprintLibrary.SetInputMode_UIOnlyEx` _returnvalue null))

(fn `LineTraceForShooting`
  (bind _gun (`self.Gun`))
  (bind _returnvalue (`SceneComponent.K2_GetComponentLocation` _gun))
  (`KismetSystemLibrary.LineTraceSingle` _returnvalue (+ _returnvalue (* (`SceneComponent.GetForwardVector` _gun) 10000)) "TraceTypeQuery1")
  (`/Engine/EditorBlueprintResources/StandardMacros.DecrementInt` (`self.Ammo`)))

(fn `TakeDamage`
  (params (Damage :type Integer))
  (bind _output_get (set `self.Lives` (- (`self.Lives`) Damage)))
  (`/Game/Resource/HUD/WB_PaperHUD.UpdateLives` (`self.HUD`) _output_get)
  (if (== _output_get 0)
    (`Widget.SetVisibility` (`/Game/Resource/HUD/WB_PaperHUD.GameOverScreen` (`self.HUD`)) "Visible")
    (`self.DeathOperation`)
    (else
      (`KismetSystemLibrary.PrintString` (`KismetStringLibrary.Conv_IntToString` _output_get)))))

(fn `UserConstructionScript`)